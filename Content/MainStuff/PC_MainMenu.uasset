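; Player controller for the main menu that builds the menu UI when play begins.
; For the local controller only, it creates and caches widgets for the menu chooser, multiplayer menu, server creation, server browser, skin selection, settings and private room password.
; Only the chooser is added to the viewport, with UI-only input focused on it and the mouse locked.
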(event EventBeginPlay
  (if (Pawn|IsLocalPlayerController)
    (bind _returnvalue (UserInterface|CreateWidget "/Game/UIAndWidgets/UI_MainMenuMultiplayer.UI_MainMenuMultiplayer_C"))
    (Variables|Default|SetMainMenuMultiplayer_Ref _returnvalue)
    (bind _returnvalue_2 (UserInterface|CreateWidget "/Game/UIAndWidgets/UI_CreateServer.UI_CreateServer_C"))
    (Variables|Default|SetCreateServer_Ref _returnvalue_2)
    (bind _returnvalue_3 (UserInterface|CreateWidget "/Game/UIAndWidgets/UI_ServerBrowser.UI_ServerBrowser_C"))
    (Variables|Default|SetUI_ServerBrowser_Ref _returnvalue_3)
    (bind _returnvalue_4 (UserInterface|CreateWidget "/Game/UIAndWidgets/UI_MainMenuChoose.UI_MainMenuChoose_C"))
    (bind _output_get (Variables|Default|SetMainMenuChoose_Ref _returnvalue_4))
    (UserInterface|Viewport|AddtoViewport _output_get 0)
    (Input|SetInputModeUIOnly (Game|GetPlayerController 0) _output_get "LockAlways" false)
    (bind _returnvalue_5 (UserInterface|CreateWidget "/Game/UIAndWidgets/UI_ChooseSkin.UI_ChooseSkin_C"))
    (Variables|Default|SetUI_ChooseSkin_Ref _returnvalue_5)
    (bind _returnvalue_6 (UserInterface|CreateWidget "/Game/UIAndWidgets/UI_Settings.UI_Settings_C"))
    (Variables|Default|SetUI_Settings_Ref _returnvalue_6)
    (bind _returnvalue_7 (UserInterface|CreateWidget "/Game/UIAndWidgets/UI_PrivateRoomPasword.UI_PrivateRoomPasword_C"))
    (Variables|Default|SetUI_PrivateRoomPassword_Ref _returnvalue_7)))

(fn ConstructionScript)